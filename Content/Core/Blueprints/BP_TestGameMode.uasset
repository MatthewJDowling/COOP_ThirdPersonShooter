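; Test game mode that spawns enemy bots and awards score for kills of non-player pawns.
; SpawnNewBot runs an EQS query for a spawn location, then spawns either a shooter pawn or a tracker bot there at weighted random, favoring the shooter.
; On BeginPlay it binds to OnActorKilled, adding points to the killer's SPlayerState when an AI pawn dies and printing the new score.
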(event Custom|OnQueryFinishedEvent_Event_0
  (params (QueryInstance :type Env%20Query%20Instance%20Blueprint%20Wrapper%20Object%20Reference) (QueryStatus :type EEnvQueryStatus%20Enum :default "Processing"))
  (switch Utilities|FlowControl|Switch|SwitchonEEnvQueryStatus QueryStatus
    (:Success
      (for _array_element (Class|EnvQueryInstanceBlueprintWrapper|GetResultsasLocations QueryInstance)
        (Game|SpawnActorfromClass (select (not (> (Math|Random|RandomFloatinRange 0.0 1e+02) 6e+01)) "/Game/ShooterAI/AI_ShooterPawn.AI_ShooterPawn_C" "/Game/TrackerBot/BP_STrackerBot.BP_STrackerBot_C") (Math|Transform|MakeTransform _array_element) "AdjustIfPossibleButDontSpawnIfColliding" 0 0)))))

(event Custom|OnActorKilled_Event_0
  (params (VictimActor :type Actor%20Object%20Reference) (KillerActor :type Actor%20Object%20Reference) (KillerController :type Controller%20Object%20Reference))
  (bind _aspawn (Utilities|Casting|CastToPawn VictimActor))
  (if (not (Pawn|IsPlayerControlled _aspawn))
    (bind _assplayer_state (Utilities|Casting|CastToSPlayerState (Variables|/Script/Engine.Pawn|GetPlayerState (Pawn|GetControlledPawn KillerController))))
    (Class|SPlayerState|AddScore _assplayer_state 2e+01)
    (Development|PrintString (Utilities|String|ToString(Float) (Variables|/Script/Engine.PlayerState|GetScore _assplayer_state)))))

(event EventBeginPlay
  (EventDispatchers|AssignOnActorKilled (delegate Custom|OnActorKilled_Event_0)))

(event EventSpawnNewBot
  (bind _returnvalue (AI|EQS|RunEQSQuery "/Game/TrackerBot/EQS_FindSpawnLocation.EQS_FindSpawnLocation" self "RandomBest25Pct"))
  (EventDispatchers|AssignOnQueryFinishedEvent _returnvalue (delegate Custom|OnQueryFinishedEvent_Event_0)))

(fn ConstructionScript)