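; BP_SCharacter is a player character Blueprint that sets up the HUD and captures weapon input.
; On BeginPlay, a locally controlled instance creates crosshair and health indicator widgets and adds them to the player screen.
; Fire and Reload input toggle the FireButtonDown and IsReloading flags on press and release, with no firing or reload logic in this graph.
; An unconnected check that would clear FireButtonDown when CurrentWeapon has no ammo never runs.
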(event EventBeginPlay
  (if (Pawn|IsLocallyControlled)
    (Utilities|FlowControl|Sequence
      (:then_0
        (bind _returnvalue (UserInterface|CreateWidget "/Game/UI/WBP_Crosshair.WBP_Crosshair_C" (Game|GetPlayerController 0)))
        (UserInterface|Viewport|AddtoPlayerScreen _returnvalue))
      (:then_1
        (bind _returnvalue_2 (UserInterface|CreateWidget "/Game/UI/WBP_HealthIndicator.WBP_HealthIndicator_C" (Game|GetPlayerController 0)))
        (UserInterface|Viewport|AddtoPlayerScreen _returnvalue_2)))))

(event Collision|EventActorBeginOverlap
  (params (OtherActor :type Actor%20Object%20Reference)))

(event Input|ActionEvents|InputActionFire
  (params (Key :type Key%20Structure))
  (:Pressed
    (Variables|Default|SetFireButtonDown true))
  (:Released
    (Variables|Default|SetFireButtonDown false)))

(event Input|ActionEvents|InputActionReload
  (params (Key :type Key%20Structure))
  (:Pressed
    (Variables|Default|SetIsReloading true))
  (:Released
    (Variables|Default|SetIsReloading false)))

(fn ConstructionScript)